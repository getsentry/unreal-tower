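; Sentry tower projectile variant that slows enemies.
; It implements ApplySpecialEffect, acting only on SentryTowerEnemyBase actors, and multiplies their FloatingPawnMovement max speed by SlowDebuff.
; The change has no timer or reset here, so repeated applications to the same enemy compound.
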(event EventBeginPlay
  (|CallParentFunction) ; This node is disabled and will not be called.\nDrag off pins to build functionality.
)

(event Collision|EventActorBeginOverlap
  (params (OtherActor :type Actor%20Object%20Reference))
  (|CallParentFunction OtherActor) ; This node is disabled and will not be called.\nDrag off pins to build functionality.
)

(event EventTick
  (params (DeltaSeconds :type Float%20%28single-precision%29))
  (|CallParentFunction DeltaSeconds) ; This node is disabled and will not be called.\nDrag off pins to build functionality.
)

(event EventApplySpecialEffect
  (params (OtherActor :type Actor%20Object%20Reference))
  (bind _assentry_tower_enemy_base (Utilities|Casting|CastToSentryTowerEnemyBase OtherActor))
  (Variables|/Script/Engine.FloatingPawnMovement|SetMaxSpeed (.AsFloating%20Pawn%20Movement (Utilities|Casting|CastToFloatingPawnMovement (Pawn|GetMovementComponent _assentry_tower_enemy_base))) (* (Class|MovementComponent|GetMaxSpeed (.AsFloating%20Pawn%20Movement (Utilities|Casting|CastToFloatingPawnMovement (Pawn|GetMovementComponent _assentry_tower_enemy_base)))) (Variables|Default|GetSlowDebuff))))

(fn ConstructionScript
  (|CallParentFunction))